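; AI controller for a turret that keeps track of which actors it can currently see.
; The perception component's target update event filters stimuli to the sight sense.
; Sensed actors are added uniquely to a target list, and actors that drop out of sight are removed through a helper function.
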(event `self.AIPerception.OnTargetPerceptionUpdated`
  (params (Actor :type "Actor Object Reference") (Stimulus :type "AIStimulus Structure"))
  (bind _returnvalue (`AIPerceptionSystem.GetSenseClassForStimulus` Stimulus))
  (if (== _returnvalue "/Script/AIModule.AISense_Sight")
    (if (`.bSuccessfullySensed` (break `AIStimulus` Stimulus))
      (`KismetArrayLibrary.Array_AddUnique` (`self.All_Traget_Actores`) Actor)
      (else
        (`self.Remove_Target_Actor` Actor)))))

(fn `Remove_Target_Actor`
  (params (Target_Actor :type "Actor Object Reference (by ref)"))
  (`KismetArrayLibrary.Array_RemoveItem` (`self.All_Traget_Actores`) Target_Actor))

(fn `UserConstructionScript`)